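; Player character Blueprint that switches a level-based mode through the Gameplay Ability System and opens the pause screen.
; Number keys and mouse wheel call ChangeMode, which clamps the value, applies GE_SetLevel with a SetByCaller magnitude, then plays a Niagara effect and sound.
; The pause input async-loads the widget class before adding it to the viewport.
; A debug key prints the locked target, and Recovery is an empty stub.
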(event Input|EnhancedActionEvents|EnhancedInputActionIA_PauseMenu
  (params (ActionValue :type Boolean) (ElapsedSeconds :type Float%20%28double-precision%29) (TriggeredSeconds :type Float%20%28double-precision%29) (InputAction :type Input%20Action%20Object%20Reference :default "/Game/PlayerCharcter/Input/Actions/IA_PauseMenu.IA_PauseMenu"))
  (:Started
    (bind _class (Utilities|AsyncLoadClassAsset "/Game/Widgets/GameModeWidgets/WBP_PauseScreen.WBP_PauseScreen_C")
      (:Completed
        (bind _asuser_widget (Utilities|Casting|CastToUserWidgetClass _class))
        (bind _returnvalue (UserInterface|CreateWidget _asuser_widget))
        (UserInterface|Viewport|AddtoViewport _returnvalue 0)))))

(event Collision|EventActorBeginOverlap
  (params (OtherActor :type Actor%20Object%20Reference)))

(event EventTick
  (params (DeltaSeconds :type Float%20%28single-precision%29)))

(event Input|KeyboardEvents|0
  (params (Key :type Key%20Structure :default "None"))
  (bind _lockedtarget (Variables|Default|GetLockedTarget))
  (:Pressed
    (Utilities|IsValid _lockedtarget
      (:Is%20Valid
        (Development|PrintString (Utilities|GetDisplayName _lockedtarget)))
      (:Is%20Not%20Valid
        (Development|PrintString "Not Valid")))))

(event Input|KeyboardEvents|4
  (params (Key :type Key%20Structure :default "None"))
  (:Pressed
    (CallFunction|ChangeMode 3)))

(event Input|MouseEvents|MouseWheelUp
  (params (Key :type Key%20Structure :default "None"))
  (:Pressed
    (CallFunction|ChangeMode (Math|Float|Truncate (+ (.ReturnValue (Class|AbilitySystemComponent|GetGameplayAttributeValue (Variables|Default|GetPlayerAbilitySystemComponent) "(AttributeName=\"Level\",Attribute=/Script/MAV_BossFight.PlayerAttributeSet:Level,AttributeOwner=\"/Script/CoreUObject.Class'/Script/MAV_BossFight.PlayerAttributeSet'\")")) 1.0)))))

(event Input|MouseEvents|MouseWheelDown
  (params (Key :type Key%20Structure :default "None"))
  (:Pressed
    (CallFunction|ChangeMode (Math|Float|Truncate (+ (.ReturnValue (Class|AbilitySystemComponent|GetGameplayAttributeValue (Variables|Default|GetPlayerAbilitySystemComponent) "(AttributeName=\"Level\",Attribute=/Script/MAV_BossFight.PlayerAttributeSet:Level,AttributeOwner=\"/Script/CoreUObject.Class'/Script/MAV_BossFight.PlayerAttributeSet'\")")) -1.0)))))

(event Input|KeyboardEvents|1
  (params (Key :type Key%20Structure :default "None"))
  (:Pressed
    (CallFunction|ChangeMode)))

(event Input|KeyboardEvents|2
  (params (Key :type Key%20Structure :default "None"))
  (:Pressed
    (CallFunction|ChangeMode 1)))

(event Input|KeyboardEvents|3
  (params (Key :type Key%20Structure :default "None"))
  (:Pressed
    (CallFunction|ChangeMode 2)))

(fn ConstructionScript)

(fn ChangeMode
  (params (ChangeModeTo :type Integer))
  (bind _returnvalue (Transformation|GetActorLocation))
  (bind _returnvalue_2 (Ability|GameplayEffect|AssignTagSetbyCallerMagnitude (GameplayEffects|MakeOutgoingSpec :self (Variables|Default|GetPlayerAbilitySystemComponent) :GameplayEffectClass "/Game/EnemyCharacter/Triceratops/GameplayEffect/GE_SetLevel.GE_SetLevel_C") "(TagName=\"Data.Level\")" (Math|Conversions|ToFloat(Integer) (Math|Integer|Clamp(Integer) ChangeModeTo 1 4))))
  (GameplayEffects|ApplyGameplayEffectSpecToSelf (Variables|Default|GetPlayerAbilitySystemComponent) _returnvalue_2)
  (Niagara|SpawnSystematLocation "/Game/Assets/niagara/NewNiagaraSystem1.NewNiagaraSystem1" (Math|Vector|MakeVector (.x _returnvalue) (.y _returnvalue) (+ (.z _returnvalue) 5e+01)) "0, 0, 0" "0.500000,0.500000,0.500000")
  (Audio|PlaySound2D "/Game/Assets/Sounds/SW_Ding_1.SW_Ding_1" 1.0 1.0 0.0 0 0))

(fn Recovery)