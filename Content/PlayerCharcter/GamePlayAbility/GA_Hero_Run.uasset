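; GA_Hero_Run is a gameplay ability that makes the player character run.
; On activation it applies the GE_Run effect, caches the current max walk speed, and raises the movement component's speed to RunningSpeed.
; When the ability ends, it restores the cached speed and removes the effect through its stored handle.
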(event Ability|EventActivateAbility
  (bind _asplayer_character (Utilities|Casting|CastToPlayerCharacter (Ability|GetAvatarActorfromActorInfo)))
  (bind _returnvalue (Ability|ApplyGameplayEffectToOwner "/Game/PlayerCharcter/GamePlayEffect/GE_Run.GE_Run_C"))
  (Variables|Default|SetActivedEffect _returnvalue)
  (Variables|Default|SetWalkingSpeed (Variables|/Script/Engine.CharacterMovementComponent|GetMaxWalkSpeed (Variables|/Script/Engine.Character|GetCharacterMovement _asplayer_character)))
  (Variables|/Script/Engine.CharacterMovementComponent|SetMaxWalkSpeed (Variables|/Script/Engine.Character|GetCharacterMovement _asplayer_character) (Variables|Default|GetRunningSpeed)))

(event Ability|EventOnEndAbility
  (params (bWasCancelled :type Boolean))
  (Variables|/Script/Engine.CharacterMovementComponent|SetMaxWalkSpeed (Variables|/Script/Engine.Character|GetCharacterMovement (stale Ability|EventActivateAbility _asplayer_character)) (Variables|Default|GetWalkingSpeed))
  (Ability|RemoveGameplayEffectFromOwnerWithHandle (Variables|Default|GetActivedEffect)))