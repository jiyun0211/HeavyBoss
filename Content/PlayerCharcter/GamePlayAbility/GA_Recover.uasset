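; GA_Recover is a player gameplay ability that performs a directional recovery move, gated by an equality check between two avatar attributes.
; It turns the last movement input into the RollingDirection motion-warp rotation, then plays the recovery montage sped up.
; Completion or blend-out applies GE_Recovery with a stamina change through a spec handle and ends on success.
; Interruption, cancellation or a failed check ends the ability without the effect.
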(event Ability|EventOnEndAbility
  (params (bWasCancelled :type Boolean)))

(event Ability|EventActivateAbility
  (bind _returnvalue (Ability|GetAvatarActorfromActorInfo))
  (if (== (.ReturnValue (Ability|Attribute|GetFloatAttribute _returnvalue "(AttributeName=\"MaxCool\",Attribute=/Script/MAV_BossFight.PlayerAttributeSet:MaxCool,AttributeOwner=\"/Script/CoreUObject.Class'/Script/MAV_BossFight.PlayerAttributeSet'\")")) (.ReturnValue (Ability|Attribute|GetFloatAttribute _returnvalue "(AttributeName=\"RecoveryCool\",Attribute=/Script/MAV_BossFight.PlayerAttributeSet:RecoveryCool,AttributeOwner=\"/Script/CoreUObject.Class'/Script/MAV_BossFight.PlayerAttributeSet'\")")))
    (CallFunction|Direction)
    (|PlayMontageandWaitProxy "None" "/Game/PlayerCharcter/Montage/AM_Recovery.AM_Recovery" 1.5 "None" true 1.0 0.0 false
      (:OnCompleted
        (Class|PlayerGameplayAbility|ApplyEffectSpecHandletoTarget (Ability|GetAvatarActorfromActorInfo) (Class|PlayerHeroGameplayAbility|MakePlayerStaminaEffectSpecHandle "/Game/PlayerCharcter/GamePlayEffect/GE_Recovery.GE_Recovery_C" 3e+01) :!label _label
          (:Successful
            _)))
      (:OnBlendOut
        (goto _label))
      (:OnInterrupted
        _)
      (:OnCancelled
        _))
    (Ability|EndAbility)
    (else
      (Ability|EndAbility))))

(fn Direction
  (Variables|Default|SetCachedRollingDirection (Math|Vector|Normalize (Class|Pawn|GetLastMovementInputVector (Class|PlayerGameplayAbility|GetPlayerCharacterfromActorInfo))))
  (Utilities|FlowControl|Sequence
    (:then_0
      (Class|MotionWarpingComponent|AddorUpdateWarpTargetfromLocationandRotation (Variables|/Script/MAV_BossFight.PlayerBaseCharacter|GetMotionWarpingComponent (Class|PlayerGameplayAbility|GetPlayerCharacterfromActorInfo)) "RollingDirection" "0, 0, 0" (Math|Rotator|MakeRotfromX (Variables|Default|GetCachedRollingDirection))))))