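; GA_Roll is a player roll Gameplay Ability, currently unfinished: activation only prints a string.
; Its disconnected roll chain calls Direction, plays AM_Roll at increased speed and ends the ability on any montage outcome.
; Direction caches the normalized last movement input and feeds it as rotation to the RollingDirection Motion Warping target, with a zero location.
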(event Ability|EventActivateAbility
  (Development|PrintString "Hello"))

(event Ability|EventOnEndAbility
  (params (bWasCancelled :type Boolean)))

(fn Direction
  (Variables|Default|SetCachedRollingDirection (Math|Vector|Normalize (Class|Pawn|GetLastMovementInputVector (Class|PlayerGameplayAbility|GetPlayerCharacterfromActorInfo))))
  (Utilities|FlowControl|Sequence
    (:then_0
      (Class|MotionWarpingComponent|AddorUpdateWarpTargetfromLocationandRotation (Variables|/Script/MAV_BossFight.PlayerBaseCharacter|GetMotionWarpingComponent (Class|PlayerGameplayAbility|GetPlayerCharacterfromActorInfo)) "RollingDirection" "0, 0, 0" (Math|Rotator|MakeRotfromX (Variables|Default|GetCachedRollingDirection))))))