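; BP_Triceratops is the triceratops enemy character, with an eye color that changes by mode level.
; BeginPlay forces walking movement, runs the parent logic, then creates a dynamic material instance on mesh element 1 for the eyes.
; The ChangeModeColor event uses the given level to index the Colors array and writes that color into the eye material.
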(event Custom|ChangeModeColor
  (params (level :type Integer))
  (Rendering|Material|SetVectorParameterValue (Variables|Default|GetEyeMaterial) "BaseCOlor" (Math|Conversions|ToLinearColor(Color) (Utilities|Array|Get(acopy) (Variables|Default|GetColors) level)) :!class /Script/Engine.MaterialInstanceDynamic))

(event EventBeginPlay
  (Pawn|Components|CharacterMovement|SetMovementMode (Variables|Character|GetCharacterMovement) "MOVE_Walking" 0)
  (|CallParentFunction)
  (bind _returnvalue (Rendering|Material|CreateDynamicMaterialInstance (Variables|Character|GetMesh) 1 "/Game/Assets/Enemies/Dinosaur/Material_002_Inst.Material_002_Inst" "None" :!class /Script/Engine.PrimitiveComponent))
  (Variables|Default|SetEyeMaterial _returnvalue))

(event Collision|EventActorBeginOverlap
  (params (OtherActor :type Actor%20Object%20Reference))
  (|CallParentFunction OtherActor) ; This node is disabled and will not be called.\nDrag off pins to build functionality.
)

(fn ConstructionScript
  (|CallParentFunction))