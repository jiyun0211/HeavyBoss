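; Gameplay Ability that switches the Triceratops enemy to a random mode.
; It applies GE_SetLevel to the avatar, passing a random integer level from a small range as a SetByCaller magnitude under Data.Level.
; On success it plays a ding, prints a float attribute read from the avatar and passes it truncated to BP_Triceratops.ChangeModeColor.
; Debug prints report the result, and the ability calls EndAbility without waiting.
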(event Ability|EventActivateAbility
  (bind _returnvalue (Ability|GetAvatarActorfromActorInfo))
  (bind _returnvalue_2 (Ability|Attribute|GetFloatAttribute _returnvalue "(AttributeName=\"Level\",Attribute=/Script/MAV_BossFight.PlayerAttributeSet:Level,AttributeOwner=\"/Script/CoreUObject.Class'/Script/MAV_BossFight.PlayerAttributeSet'\")"))
  (bind _returnvalue_3 (Ability|GameplayEffect|AssignTagSetbyCallerMagnitude (Ability|MakeOutgoingGameplayEffectSpec "/Game/EnemyCharacter/Triceratops/GameplayEffect/GE_SetLevel.GE_SetLevel_C") "(TagName=\"Data.Level\")" (Math|Conversions|ToFloat(Integer) (Math|Random|RandomIntegerinRange 1 4))))
  (Class|PlayerGameplayAbility|ApplyEffectSpecHandletoTarget (Ability|GetAvatarActorfromActorInfo) _returnvalue_3
    (:Successful
      (Development|PrintString (Utilities|String|ToString(Float) _returnvalue_2))
      (Audio|PlaySound2D "/Game/Assets/Sounds/SW_Ding_1.SW_Ding_1" 1.0 1.0 0.0 0 0)
      (bind _asbp_triceratops (Utilities|Casting|CastToBP_Triceratops (Ability|GetAvatarActorfromActorInfo))
        (:then
          (Default|ChangeModeColor _asbp_triceratops (Math|Float|Truncate _returnvalue_2)))
        (:CastFailed
          _)))
    (:Failed
      (Development|PrintString "Fail")))
  (Ability|EndAbility))

(event Ability|EventOnEndAbility
  (params (bWasCancelled :type Boolean)))